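; AI controller for enemy NPCs built on the Sandbox CMC character, translating AI decisions into pawn actions and handling death.
; ApplyLocomotionIntent writes the gait, strafe, aim and crouch input state, syncing crouch when it changes, while Fireat forwards an aim point to the pawn.
; Tick polls health and, at zero, sets the blackboard death key, flags the AnimBP dead and starts ragdoll.
; BPCanFire is a stub that always returns false.
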(event `self.BP_ApplyLocomotionIntent`
  (params (bWantsWalk :type Boolean) (bWantsSprint :type Boolean) (bWantsStrafe :type Boolean) (bWantsAim :type Boolean) (bWantsCrouch :type Boolean))
  (bind _assandbox_character_cmc_npc_enemy (cast `/Game/MyStuff/AI/Enemy/SandboxCharacter_CMC_NPC_Enemy` (`self.K2_GetPawn`)))
  (bind _output_get (set `/Game/Blueprints/SandboxCharacter_CMC.CharacterInputState` (make `/Game/Blueprints/Data/S_PlayerInputState` bWantsSprint bWantsWalk bWantsStrafe bWantsAim bWantsCrouch) _assandbox_character_cmc_npc_enemy))
  (bind (_wantstosprint _wantstowalk _wantstostrafe _wantstoaim _wantstocrouch) (break `/Game/Blueprints/Data/S_PlayerInputState` _output_get))
  (if (!= _wantstocrouch (`Character.bIsCrouched` _assandbox_character_cmc_npc_enemy))
    (if _wantstocrouch
      (`Character.Crouch` _assandbox_character_cmc_npc_enemy)
      (else
        (`Character.UnCrouch` _assandbox_character_cmc_npc_enemy)))))

(event `self.BP_FireAt`
  (params (AimPoint :type "Vector Structure (by ref)"))
  (bind _assandbox_character_cmc_npc_enemy (cast `/Game/MyStuff/AI/Enemy/SandboxCharacter_CMC_NPC_Enemy` (`self.K2_GetPawn`)))
  (`/Game/MyStuff/AI/Enemy/SandboxCharacter_CMC_NPC_Enemy.FireAtLocation` _assandbox_character_cmc_npc_enemy AimPoint))

(event `self.ReceiveTick`
  (params (DeltaSeconds :type "Float (single-precision)"))
  (bind _assandbox_character_cmc (cast `/Game/Blueprints/SandboxCharacter_CMC` (`self.K2_GetPawn`)))
  (bind _assandbox_character_cmc_abp (cast `/Game/Blueprints/SandboxCharacter_CMC_ABP` (`SkeletalMeshComponent.GetAnimInstance` (`Character.Mesh` _assandbox_character_cmc))))
  (if (`/Game/Blueprints/SandboxCharacter_CMC_ABP.bIsDead` _assandbox_character_cmc_abp)
    _
    (elif (<= (`HealthComponent.CurrentHealth` (`/Game/Blueprints/SandboxCharacter_CMC.Health` _assandbox_character_cmc)) 0.0)
      (`BlackboardComponent.SetValueAsBool` (`AIBlueprintHelperLibrary.GetBlackboard` null) (`self.Key_IsDead`) true)
      (set `/Game/Blueprints/SandboxCharacter_CMC_ABP.bIsDead` true _assandbox_character_cmc_abp)
      (`/Game/Blueprints/SandboxCharacter_CMC.Ragdoll_Start` _assandbox_character_cmc))))

(fn `BP_CanFire`
  (returns (ReturnValue :type Boolean))
  (return false))

(fn `UserConstructionScript`)